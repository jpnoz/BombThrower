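; Player character Blueprint that picks up, puts down and throws interactables, including bombs, and passes damage to a health component.
; Input actions set Play animation flags on the animation control component, with pick-up first box-tracing ahead for an InteractableBase target.
; Tick polls the matching Run flags to call the interaction component, then resets flags and clears the target on release.
; A fallback lets the arms lower when a held bomb explodes.
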(event Input|EnhancedActionEvents|EnhancedInputActionIA_PickUp
  (params (ActionValue :type Boolean) (ElapsedSeconds :type Float%20%28double-precision%29) (TriggeredSeconds :type Float%20%28double-precision%29) (InputAction :type Input%20Action%20Object%20Reference :default "/Game/Input/Actions/IA_PickUp.IA_PickUp"))
  (bind _returnvalue (Transformation|GetActorLocation))
  (:Started
    (bind (_traceresult _returnvalue_2) (Class|BTInteractionComponent|BBoxTrace (Variables|Default|GetInteractionComponent) _returnvalue (+ _returnvalue (* (Transformation|GetActorForwardVector) (Variables|/Script/BombThrow.BTMovementComponent|GetSurfaceDetectionRange (Variables|Default|GetMovementComponent))))))
    (if (and _returnvalue_2 (Class|GameplayStatics|ObjectIsA (.HitActor (Collision|BreakHitResult _traceresult)) "/Script/BombThrow.InteractableBase"))
      (Variables|Default|SetTarget%20Interactable (.HitActor (Collision|BreakHitResult _traceresult)))
      (Class|BTAnimationControlComponent|SetAnimationFlag (Variables|Default|GetAnimationControlComponent) "PlayPickUp" true))))

(event Input|EnhancedActionEvents|EnhancedInputActionIA_Throw
  (params (ActionValue :type Boolean) (ElapsedSeconds :type Float%20%28double-precision%29) (TriggeredSeconds :type Float%20%28double-precision%29) (InputAction :type Input%20Action%20Object%20Reference :default "/Game/Input/Actions/IA_Throw.IA_Throw"))
  (:Started
    (Class|BTAnimationControlComponent|SetAnimationFlag (Variables|Default|GetAnimationControlComponent) "PlayThrow" (Utilities|IsValid (Variables|Default|GetTarget%20Interactable)))))

(event Input|EnhancedActionEvents|EnhancedInputActionIA_PutDown
  (params (ActionValue :type Boolean) (ElapsedSeconds :type Float%20%28double-precision%29) (TriggeredSeconds :type Float%20%28double-precision%29) (InputAction :type Input%20Action%20Object%20Reference :default "/Game/Input/Actions/IA_PutDown.IA_PutDown"))
  (:Started
    (Class|BTAnimationControlComponent|SetAnimationFlag (Variables|Default|GetAnimationControlComponent) "PlayPutDown" true)))

(event EventBeginPlay
  (bind _returnvalue (Game|GetPlayerCameraManager 0))
  (bind _characterinputcomponent (Variables|Default|GetCharacterInputComponent))
  (Variables|/Script/Engine.PlayerCameraManager|SetViewPitchMin _returnvalue (* (Variables|/Script/BombThrow.BTCharacterInputComponent|GetMaxPitch _characterinputcomponent) -1.0))
  (Variables|/Script/Engine.PlayerCameraManager|SetViewPitchMax _returnvalue (* (Variables|/Script/BombThrow.BTCharacterInputComponent|GetMinPitch _characterinputcomponent) -1.0)))

(event Collision|EventActorBeginOverlap
  (params (OtherActor :type Actor%20Object%20Reference)))

(event EventTick
  (params (DeltaSeconds :type Float%20%28single-precision%29))
  (bind _interactioncomponent (Variables|Default|GetInteractionComponent))
  (bind _animationcontrolcomponent (Variables|Default|GetAnimationControlComponent))
  (bind _animationcontrolcomponent_2 (Variables|Default|GetAnimationControlComponent))
  (bind _animationcontrolcomponent_3 (Variables|Default|GetAnimationControlComponent))
  (bind _returnvalue (Class|BTAnimationControlComponent|BGetAnimationFlag _animationcontrolcomponent_2 "RunPickUp"))
  ;[0.102 0.102 0.102] Ugly separate ifs
  (if (and _returnvalue (Utilities|IsValid (Variables|Default|GetTarget%20Interactable)))
    (Class|BTInteractionComponent|PickUpInteractable _interactioncomponent (Variables|Default|GetTarget%20Interactable))
    (Class|BTAnimationControlComponent|SetAnimationFlag _animationcontrolcomponent_3 "PlayPickUp" false)
    (Class|BTAnimationControlComponent|SetAnimationFlag _animationcontrolcomponent_3 "RunPickUp" false)
    (else
      (bind _returnvalue_2 (Class|BTAnimationControlComponent|BGetAnimationFlag _animationcontrolcomponent_2 "RunPutDown"))
      (if _returnvalue_2
        (Class|BTInteractionComponent|PutDownInteractable _interactioncomponent)
        (Class|BTAnimationControlComponent|SetAnimationFlag _animationcontrolcomponent_3 "PlayPutDown" false)
        (Class|BTAnimationControlComponent|SetAnimationFlag _animationcontrolcomponent_3 "RunPutDown" false)
        ;[0.102 0.102 0.102 1 12] Reset Held Interactable after releasing
        (Variables|Default|SetTarget%20Interactable 0 :!label _label)
        (else
          (bind _returnvalue_3 (Class|BTAnimationControlComponent|BGetAnimationFlag _animationcontrolcomponent_2 "RunThrow"))
          (if _returnvalue_3
            (Class|BTInteractionComponent|ThrowInteractable _interactioncomponent)
            (Class|BTAnimationControlComponent|SetAnimationFlag _animationcontrolcomponent_3 "PlayThrow" false)
            (Class|BTAnimationControlComponent|SetAnimationFlag _animationcontrolcomponent_3 "RunThrow" false)
            (goto _label)
            (else
              ;[0.1 0.1 0.1] Allow player to put down arms when held bomb explodes
              (bind _returnvalue_4 (Class|BTAnimationControlComponent|BGetAnimationFlag _animationcontrolcomponent "PlayPutDown"))
              (if (and (not (Utilities|IsValid (Variables|Default|GetTarget%20Interactable))) _returnvalue_4)
                (Class|BTAnimationControlComponent|SetAnimationFlag _animationcontrolcomponent "PlayPickUp" false)
                (Class|BTAnimationControlComponent|SetAnimationFlag _animationcontrolcomponent "RunPutDown" true)))))))))

(event Game|Damage|EventAnyDamage
  (params (Damage :type Float%20%28single-precision%29) (DamageType :type Damage%20Type%20Object%20Reference) (InstigatedBy :type Controller%20Object%20Reference) (DamageCauser :type Actor%20Object%20Reference))
  (bind _healthcomponent (Variables|Default|GetHealthComponent))
  (Class|BTHealthComponent|TakeDamage _healthcomponent Damage)
  (Development|PrintString (Utilities|String|ToString(Integer) (Variables|/Script/BombThrow.BTHealthComponent|GetCurrentHealth _healthcomponent)) true true "(R=0.348958,G=0.007839,B=0.000000,A=1.000000)"))

(fn ConstructionScript)