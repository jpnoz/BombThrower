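; Game state Blueprint that tracks defend objectives, players and enemies, and ends the round when a loss or win condition is met.
; Defeat and destruction events remove the actor from its list and print debug text.
; Any destroyed objective, or an emptied player or enemy list, leads to a shared delayed reset that reopens TestLevel, with no distinction between winning and losing.
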(event EventBeginPlay)

(event EventTick
  (params (DeltaSeconds :type Float%20%28single-precision%29)))

(event EventOnDefendObjectiveDestroyed
  (params (DestroyedObjective :type Actor%20Object%20Reference))
  (Utilities|Array|RemoveItem (Variables|Default|GetAllDefendObjectives) DestroyedObjective)
  (Development|PrintString "OBJECTIVE DESTROYED" true true "(R=0.000000,G=0.250000,B=0.080202,A=1.000000)")
  (Utilities|FlowControl|Delay 1.0)
  (Development|PrintString "Resetting..." true true "(R=0.244470,G=0.000000,B=0.968750,A=1.000000)")
  (Utilities|FlowControl|Delay 5.0)
  (Game|OpenLevel(byName) "TestLevel"))

(event EventOnPlayerDefeated
  (params (DefeatedPlayer :type Actor%20Object%20Reference))
  (bind _allplayers (Variables|Default|GetAllPlayers))
  (Utilities|Array|RemoveItem _allplayers DefeatedPlayer)
  (Development|PrintString "PLAYER DEFEATED" true true "(R=0.000000,G=0.250000,B=0.080202,A=1.000000)")
  (if (<= (Utilities|Array|Length _allplayers) 0)
    (Development|PrintString "ALL PLAYERS DEFEATED" true true "(R=0.000000,G=0.510417,B=0.163746,A=1.000000)" 1e+01)
    (Utilities|FlowControl|Delay 1.0)
    (Development|PrintString "Resetting..." true true "(R=0.244470,G=0.000000,B=0.968750,A=1.000000)")
    (Utilities|FlowControl|Delay 5.0)
    (Game|OpenLevel(byName) "TestLevel")))

(event EventOnEnemyDefeated
  (params (DefeatedEnemy :type Actor%20Object%20Reference))
  (bind _allenemies (Variables|Default|GetAllEnemies))
  (Utilities|Array|RemoveItem _allenemies DefeatedEnemy)
  (Development|PrintString "ENEMY DEFEATED" true true "(R=0.000000,G=0.250000,B=0.080202,A=1.000000)")
  (if (<= (Utilities|Array|Length _allenemies) 0)
    (Development|PrintString "ALL ENEMIES DEFEATED" true true "(R=0.000000,G=0.510417,B=0.163746,A=1.000000)" 1e+01)
    (Utilities|FlowControl|Delay 1.0)
    (Development|PrintString "Resetting..." true true "(R=0.244470,G=0.000000,B=0.968750,A=1.000000)")
    (Utilities|FlowControl|Delay 5.0)
    (Game|OpenLevel(byName) "TestLevel")))

(fn ConstructionScript)